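; RedBullet is an enemy projectile that damages the player pawn when it overlaps it.
; On a hit it applies its Damage, spawns a scaled-up ExplosionPS at its sphere's transform and destroys itself.
; Damage is set through a SetDamage function, and a delay started from Tick destroys the bullet after a few seconds if it hits nothing.
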(event EventBeginPlay)

(event Collision|EventActorBeginOverlap
  (params (OtherActor :type Actor%20Object%20Reference))
  (bind _asplayer_pawn (Utilities|Casting|CastToPlayerPawn OtherActor))
  (Default|TakeDamage _asplayer_pawn (Variables|Default|GetDamage))
  (bind _returnvalue (Game|SpawnActorfromClass "/Game/MyStuff/Blueprints/Enemies/ExplosionPS.ExplosionPS_C" (Transformation|GetWorldTransform (Variables|Default|GetSphere)) "Undefined" 0 0))
  (Transformation|SetActorScale3D _returnvalue "5.000000,5.000000,5.000000")
  (Actor|DestroyActor))

(event EventTick
  (params (DeltaSeconds :type Float%20%28single-precision%29))
  (Utilities|FlowControl|Delay 3.0)
  (Actor|DestroyActor))

(fn ConstructionScript)

(fn SetDamage
  (params (NewDamage :type Float%20%28single-precision%29))
  (Variables|Default|SetDamage NewDamage))