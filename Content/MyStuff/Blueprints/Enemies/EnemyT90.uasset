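; T90 enemy, likely a tank, whose turret tracks the player while in line of sight.
; On BeginPlay it applies its HP and touch damage.
; Each tick it traces on the Camera channel from the turret pivot to the player's GunPivot, with debug drawing.
; If the player is hit, the turret rotates toward them via RInterpToConstant with a fixed DeltaTime, so turn speed depends on frame rate.
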(event EventBeginPlay
  (CallFunction|SetHP (Variables|Default|GetHP))
  (CallFunction|SetTouchDamage 1e+01))

(event Collision|EventActorBeginOverlap
  (params (OtherActor :type Actor%20Object%20Reference))
  (|CallParentFunction OtherActor))

(event EventTick
  (params (DeltaSeconds :type Float%20%28single-precision%29))
  (bind _turretpivot (Variables|Default|Getturretpivot))
  (bind _asplayer_pawn (Utilities|Casting|CastToPlayerPawn (Game|Player|GetPlayerPawn 0)))
  (bind _outhit (Collision|LineTraceByChannel (Transformation|GetWorldLocation (Variables|Default|Getturretpivot)) (Transformation|GetWorldLocation (Variables|/Game/MyStuff/Blueprints/Player/PlayerPawn.PlayerPawn_C|GetGunPivot _asplayer_pawn)) "TraceTypeQuery2" false 0 "ForOneFrame"))
  (Utilities|Casting|CastToPlayerPawn (.HitActor (Collision|BreakHitResult _outhit)))
  (Transformation|SetWorldRotation _turretpivot (Class|KismetMathLibrary|RInterptoConstant (Transformation|GetWorldRotation _turretpivot) (Math|Rotator|FindLookatRotation (Transformation|GetWorldLocation _turretpivot) (Transformation|GetWorldLocation (Variables|/Game/MyStuff/Blueprints/Player/PlayerPawn.PlayerPawn_C|GetGunPivot _asplayer_pawn))) 0.1 5.0) false false))

(fn ConstructionScript
  (|CallParentFunction))