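; Base enemy actor that loses health when hit by BlueBullet projectiles and explodes when killed.
; On overlap, it passes the bullet's damage to TakeDamage, which subtracts it from Health and returns whether health is depleted.
; On death it spawns a double-scale ExplosionPS at its own transform and destroys itself.
; A SetHP function allows Health to be set directly.
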(event EventBeginPlay)

(event Collision|EventActorBeginOverlap
  (params (OtherActor :type Actor%20Object%20Reference))
  (bind _asblue_bullet (Utilities|Casting|CastToBlueBullet OtherActor))
  (bind _dead (CallFunction|TakeDamage (Variables|/Game/MyStuff/Blueprints/Player/BlueBullet.BlueBullet_C|GetDamage _asblue_bullet)))
  (if _dead
    (bind _returnvalue (Game|SpawnActorfromClass "/Game/MyStuff/Blueprints/Enemies/ExplosionPS.ExplosionPS_C" (Transformation|GetActorTransform) "Undefined" 0 0))
    (Transformation|SetActorScale3D _returnvalue "2.000000,2.000000,2.000000")
    (Actor|DestroyActor)))

(event EventTick
  (params (DeltaSeconds :type Float%20%28single-precision%29)))

(fn ConstructionScript)

(fn SetHP
  (params (newHP :type Float%20%28single-precision%29))
  (Variables|Default|Sethealth newHP))

(fn TakeDamage
  (params (Damage :type Float%20%28single-precision%29))
  (bind _output_get (Variables|Default|Sethealth (- (Variables|Default|Gethealth) Damage)))
  (return (<= _output_get 0.0)))