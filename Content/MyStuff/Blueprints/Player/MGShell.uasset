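; MGShell is a player projectile actor, apparently a machine-gun round, that sets its damage to 1 on spawn.
; On overlap it ignores PlayerPawn and TankShell actors.
; Any other overlap spawns a half-scale BlueExplosionActor at its Sphere component's transform, then destroys the shell after a very short delay.
; The graph itself contains no movement or damage-application logic.
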(event EventBeginPlay
  (CallFunction|SetDamage 1.0))

(event Collision|EventActorBeginOverlap
  (params (OtherActor :type Actor%20Object%20Reference))
  (Utilities|Casting|CastToPlayerPawn OtherActor
    (:CastFailed
      (Utilities|Casting|CastToTankShell OtherActor
        (:CastFailed
          (bind _returnvalue (Game|SpawnActorfromClass "/Game/MyStuff/Blueprints/Player/BlueExplosionActor.BlueExplosionActor_C" (Transformation|GetWorldTransform (Variables|Default|GetSphere self)) "Undefined" 0 0))
          (Transformation|SetActorScale3D _returnvalue "0.500000,0.500000,0.500000")
          (Utilities|FlowControl|Delay 0.01)
          (Actor|DestroyActor))))))

(event EventTick
  (params (DeltaSeconds :type Float%20%28single-precision%29)))

(fn ConstructionScript
  (|CallParentFunction))