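; Player tank pawn that drives forward automatically while the player steers, aims and fires, with a game HUD on spawn.
; Tick moves DIRECTION forward, eases the hull back to straight and runs both weapon cooldowns.
; Axis inputs clamp hull yaw, lateral position and gun pitch; buttons fire single shells or held machine-gun bursts.
; TakeDamage reduces health and, on death, spawns an explosion, destroys the pawn, fades out and shows the death widget.
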(event EventBeginPlay
  (Variables|Default|Sethealth (Variables|Default|GetmaxHealth))
  (bind _returnvalue (UserInterface|CreateWidget "/Game/MyStuff/Blueprints/UI_Game.UI_Game_C"))
  (Default|SetPlayerRef _returnvalue self)
  (UserInterface|Viewport|AddtoViewport _returnvalue 0)
  (CameraFades|StartCameraFade (Game|GetPlayerCameraManager 0) 1.0 0.0 5.0 "(R=0.000000,G=0.000000,B=0.000000,A=5.000000)" false false))

(event Collision|EventActorBeginOverlap
  (params (OtherActor :type Actor%20Object%20Reference)))

(event EventTick
  (params (DeltaSeconds :type Float%20%28single-precision%29))
  (bind _tankpivot (Variables|Default|Gettankpivot))
  (if (Variables|Default|Getalive)
    (Utilities|FlowControl|Sequence
      (:then_0
        ;[1 1 1] Keep movingtank+camera
        (Transformation|AddLocalOffset (Variables|Default|GetDIRECTION) (Math|Vector|MakeVector (Variables|Default|GetTankForwardSpeed) 0.0 0.0) false false)
        ;[1 1 1] rotate tank forward
        (Transformation|SetWorldRotation _tankpivot (Math|Interpolation|RInterpTo (Transformation|GetWorldRotation _tankpivot) (Variables|Default|GetTankForwardDirection) 0.1 0.6) false false))
      (:then_1
        ;[1 1 1] main delay cooldown
        (if (> (Variables|Default|GetMainDelay) 0.0)
          (Variables|Default|SetMainDelay (- (Variables|Default|GetMainDelay) DeltaSeconds))))
      (:then_2
        ;[1 1 1] sub delay cooldown
        (if (> (Variables|Default|GetSubDelay) 0.0)
          (Variables|Default|SetSubDelay (- (Variables|Default|GetSubDelay) DeltaSeconds))))
      (:then_3
        ;[1 1 1] fire sub
        (if (Variables|Default|GetMGFire)
          (if (<= (Variables|Default|GetSubDelay) 0.0)
            (bind _returnvalue (Game|SpawnActorfromClass "/Game/MyStuff/Blueprints/Player/MGShell.MGShell_C" (Transformation|GetWorldTransform (Variables|Default|GetMG%20Shell%20Spawn)) "Undefined" 0 0))
            (Transformation|SetWorldScale3D (Variables|/Game/MyStuff/Blueprints/Player/BlueBullet.BlueBullet_C|GetSphere _returnvalue) "0.200000,0.200000,0.200000")
            (Variables|Default|SetSubDelay (Variables|Default|GetSubMaxDelay))))))))

(event Input|ActionEvents|InputActionFireButton
  (params (Key :type Key%20Structure :default "AnyKey"))
  (bind _tankshellspawn (Variables|Default|GetTankShellSpawn))
  (bind _returnvalue (Transformation|GetWorldTransform _tankshellspawn))
  ;[1 1 1] fire main weapon
  (:Pressed
    (if (<= (Variables|Default|GetMainDelay) 0.0)
      (bind _returnvalue_2 (Game|SpawnActorfromClass "/Game/MyStuff/Blueprints/Player/TankShell.TankShell_C" _returnvalue "Undefined" 0 0))
      (Transformation|SetWorldScale3D (Variables|/Game/MyStuff/Blueprints/Player/BlueBullet.BlueBullet_C|GetSphere _returnvalue_2) "1.000000,1.000000,1.000000")
      (bind _returnvalue_3 (Game|SpawnActorfromClass "/Game/MyStuff/Blueprints/Player/BlueExplosionActor.BlueExplosionActor_C" _returnvalue "Undefined" 0 0))
      (Transformation|SetWorldScale3D (Variables|/Game/MyStuff/Blueprints/Player/BlueExplosionActor.BlueExplosionActor_C|GetDefaultSceneRoot _returnvalue_3) "2.000000,2.000000,2.000000")
      (Variables|Default|SetMainDelay (Variables|Default|GetMainMaxDelay)))))

(event Input|ActionEvents|InputActionFire2Button
  (params (Key :type Key%20Structure :default "AnyKey"))
  (:Pressed
    (Variables|Default|SetMGFire true))
  (:Released
    (Variables|Default|SetMGFire false)))

(event Input|AxisEvents|InputAxisHullRight
  (params (AxisValue :type Float%20%28single-precision%29))
  (bind _returnvalue (Math|Float|Clamp(Float) AxisValue -1.0))
  (bind _tankpivot (Variables|Default|Gettankpivot))
  (bind _maxhullturnright (Variables|Default|GetmaxHullTurnRight))
  (bind _maxhullturnleft (Variables|Default|GetmaxHullTurnLeft))
  (bind _tankpivot_2 (Variables|Default|Gettankpivot))
  (bind _returnvalue_2 (Transformation|GetWorldLocation _tankpivot))
  (bind _returnvalue_3 (Transformation|GetWorldRotation _tankpivot_2))
  (bind _returnvalue_4 (* _returnvalue 1e+01))
  (bind _returnvalue_5 (Math|Vector|MakeVector 0.0 _returnvalue_4 0.0))
  (bind _yaw (Math|Rotator|BreakRotator _returnvalue_3))
  (bind _returnvalue_6 (+ _returnvalue_2 _returnvalue_5))
  (bind (_x _y _z) (Math|Vector|BreakVector _returnvalue_6))
  (if (Variables|Default|Getalive)
    (Utilities|FlowControl|Sequence
      (:then_0
        ;[1 1 1] turn tank
        (Transformation|AddLocalRotation (Variables|Default|Gettankpivot) (Math|Rotator|MakeRotator 0.0 0.0 _returnvalue) false false)
        ;[1 1 1] prevent turning past max
        (if (> _yaw _maxhullturnright)
          (Transformation|SetWorldRotation _tankpivot_2 (Math|Rotator|MakeRotator 0.0 0.0 _maxhullturnright) false false)
          (elif (< _yaw _maxhullturnleft)
            (Transformation|SetWorldRotation _tankpivot_2 (Math|Rotator|MakeRotator 0.0 0.0 _maxhullturnleft) false false))))
      (:then_1
        ;[1 1 1] move tank left and right
        (Transformation|SetWorldLocation _tankpivot (Math|Vector|MakeVector _x (Math|Float|Clamp(Float) _y -5e+02 5e+02) _z) false false)))))

(event Input|AxisEvents|InputAxisGunUp
  (params (AxisValue :type Float%20%28single-precision%29))
  (bind _gunpivot (Variables|Default|GetGunPivot))
  (bind _tankpivot (Variables|Default|Gettankpivot))
  (bind _maxgundepression (Variables|Default|GetmaxGunDepression))
  (bind _maxgunelevation (Variables|Default|GetmaxGunElevation))
  (bind _returnvalue (Transformation|GetWorldRotation _gunpivot))
  (bind _returnvalue_2 (Transformation|GetWorldRotation _tankpivot))
  (bind _pitch (Math|Rotator|BreakRotator _returnvalue))
  (bind _yaw (Math|Rotator|BreakRotator _returnvalue_2))
  (bind _returnvalue_3 (+ _yaw 9e+01))
  ;[1 1 1] turn gun
  (if (Variables|Default|Getalive)
    (Transformation|AddLocalRotation (Variables|Default|GetGunPivot) (Math|Rotator|MakeRotator 0.0 AxisValue 0.0) false false)
    ;[1 1 1] gun constraints
    (if (> _pitch _maxgunelevation)
      (Transformation|SetWorldRotation _gunpivot (Math|Rotator|MakeRotator 0.0 _maxgunelevation _returnvalue_3) false false)
      (elif (< _pitch _maxgundepression)
        (Transformation|SetWorldRotation _gunpivot (Math|Rotator|MakeRotator 0.0 _maxgundepression _returnvalue_3) false false)))))

(fn ConstructionScript)

(fn TakeDamage
  (params (Damage :type Float%20%28single-precision%29))
  (bind _output_get (Variables|Default|Sethealth (- (Variables|Default|Gethealth) Damage)))
  (bind _output_get_2 (Variables|Default|Setalive (not (<= _output_get 0.0))))
  (if (not _output_get_2)
    (bind _returnvalue (Game|SpawnActorfromClass "/Game/MyStuff/Blueprints/Player/BlueExplosionActor.BlueExplosionActor_C" (Transformation|GetWorldTransform (Variables|Default|Gettankpivot)) "Undefined" 0 0))
    (Transformation|SetActorScale3D _returnvalue "10.000000,10.000000,10.000000")
    (Actor|DestroyActor)
    (CameraFades|StartCameraFade :self (Game|GetPlayerCameraManager 0) :FromAlpha 0.0 :ToAlpha 1.0 :Duration 5.0 :bHoldWhenFinished true)
    (bind _returnvalue_2 (UserInterface|CreateWidget "/Game/MyStuff/Blueprints/PlayerDiedWidget.PlayerDiedWidget_C"))
    (UserInterface|Viewport|AddtoViewport _returnvalue_2 0)))