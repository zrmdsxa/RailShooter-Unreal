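; TankShell is a shell Blueprint that deals on-hit and splash damage and sets its hit damage on BeginPlay.
; Overlapping anything other than the PlayerPawn or an MGShell spawns a scaled-up BlueExplosionActor and enables query collision on Sphere1.
; Sphere1 acts as a momentary blast volume, applying SplashDamage to overlapped EnemyActorBase actors during a very short delay before the shell destroys itself.
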(event OnComponentBeginOverlap(Sphere1)
  (params (OverlappedComponent :type Primitive%20Component%20Object%20Reference) (OtherActor :type Actor%20Object%20Reference) (OtherComp :type Primitive%20Component%20Object%20Reference) (OtherBodyIndex :type Integer) (bFromSweep :type Boolean) (SweepResult :type Hit%20Result%20Structure%20%28by%20ref%29))
  (bind _asenemy_actor_base (Utilities|Casting|CastToEnemyActorBase OtherActor))
  (Default|TakeDamage _asenemy_actor_base (Variables|Default|GetSplashDamage)))

(event EventBeginPlay
  (CallFunction|SetDamage (Variables|Default|GetOnHitDamage)))

(event Collision|EventActorBeginOverlap
  (params (OtherActor :type Actor%20Object%20Reference))
  (Utilities|Casting|CastToPlayerPawn OtherActor
    (:CastFailed
      (Utilities|Casting|CastToMGShell OtherActor
        (:CastFailed
          (bind _returnvalue (Game|SpawnActorfromClass "/Game/MyStuff/Blueprints/Player/BlueExplosionActor.BlueExplosionActor_C" (Transformation|GetWorldTransform (Variables|Default|GetSphere self)) "Undefined" 0 0))
          (Transformation|SetActorScale3D _returnvalue "10.000000,10.000000,10.000000")
          (Collision|SetCollisionEnabled (Variables|Default|GetSphere1) "QueryOnly")
          (Utilities|FlowControl|Delay 0.01)
          (Actor|DestroyActor))))))

(event EventTick
  (params (DeltaSeconds :type Float%20%28single-precision%29)))

(fn ConstructionScript
  (|CallParentFunction))