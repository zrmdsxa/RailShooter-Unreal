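; BlueBullet is a short-lived player projectile actor that bursts into a blue explosion on contact.
; Overlapping anything other than a PlayerPawn spawns an enlarged BlueExplosionActor at the Sphere's transform and destroys the bullet.
; A Delay on Tick acts as a one-second lifetime, destroying the bullet without an explosion.
; SetDamage stores and prints a Damage value, which this Blueprint never applies itself.
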(event EventBeginPlay)

(event Collision|EventActorBeginOverlap
  (params (OtherActor :type Actor%20Object%20Reference))
  (Utilities|Casting|CastToPlayerPawn OtherActor
    (:CastFailed
      (bind _returnvalue (Game|SpawnActorfromClass "/Game/MyStuff/Blueprints/Player/BlueExplosionActor.BlueExplosionActor_C" (Transformation|GetWorldTransform (Variables|Default|GetSphere self)) "Undefined" 0 0))
      (Transformation|SetActorScale3D _returnvalue "10.000000,10.000000,10.000000")
      (Actor|DestroyActor))))

(event EventTick
  (params (DeltaSeconds :type Float%20%28single-precision%29))
  (Utilities|FlowControl|Delay 1.0)
  (Actor|DestroyActor))

(fn ConstructionScript)

(fn SetDamage
  (params (NewDamage :type Float%20%28single-precision%29))
  (bind _output_get (Variables|Default|SetDamage NewDamage))
  (Development|PrintString (Utilities|String|ToString(Float) _output_get)))